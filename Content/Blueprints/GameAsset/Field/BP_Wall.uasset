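; Outfield wall actor for the Home Run Derby game that detects when a batted ball goes over it.
; BeginPlay caches the HomerunDerby game state.
; When the OverTheWallCollision component is overlapped by an actor whose class is exactly ProjectileBall, BallWentOverTheWall sets the game state's current ball state to FenceBallDetermination.
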(event `self.ReceiveBeginPlay`
  (bind _ashomerun_derby_game_state (cast `/Game/Blueprints/States/HomerunDerby_GameState` (`GameplayStatics.GetGameState`)))
  (set `self.CurrentGameState` _ashomerun_derby_game_state))

(event `self.ReceiveActorBeginOverlap`
  (params (OtherActor :type "Actor Object Reference")))

(event `self.OverTheWallCollision.OnComponentBeginOverlap`
  (params (OtherActor :type "Actor Object Reference") (OtherComp :type "PrimitiveComponent Object Reference") (OtherBodyIndex :type Integer) (bFromSweep :type Boolean) (SweepResult :type "HitResult Structure (by ref)"))
  (`self.BallWentOverTheWall` OtherActor))

(event `self.ReceiveTick`
  (params (DeltaSeconds :type "Float (single-precision)")))

(fn `BallWentOverTheWall`
  (params (Object :type "Object Object Reference"))
  (if (== (`GameplayStatics.GetObjectClass` Object) "/Game/Blueprints/GameAsset/Ball/ProjectileBall.ProjectileBall_C")
    (set `/Game/Blueprints/States/HomerunDerby_GameState.ECurrentBallState` (`self.FenceBallDetermination`) (`self.CurrentGameState`)))
  (return))

(fn `UserConstructionScript`)