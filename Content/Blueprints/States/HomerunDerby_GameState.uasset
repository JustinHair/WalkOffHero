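; HomerunDerby_GameState is the game state for a home run derby mode, tracking the current ball state and home run total.
; On BeginPlay it caches the HomerunDerby game mode and copies its default ball state and starting total.
; Tick polls the ball state; on Homerun it increments the total, resets the state to AtBatInProgress and prints the new count on screen.
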(event `self.ReceiveBeginPlay`
  (bind _ashomerun_derby_game_mode (cast `/Game/Blueprints/States/HomerunDerby_GameMode` (`GameplayStatics.GetGameMode`)))
  (set `self.GameMode` _ashomerun_derby_game_mode)
  (set `self.ECurrentBallState` (`/Game/Blueprints/States/HomerunDerby_GameMode.EDefaultBallState` (`self.GameMode`)))
  (set `self.CurrentHomeRunTotal` (`/Game/Blueprints/States/HomerunDerby_GameMode.HomerunTotal` (`self.GameMode`))))

(event `self.ReceiveTick`
  (params (DeltaSeconds :type "Float (single-precision)"))
  (switch `/Game/Blueprints/States/EStateOfTheBall` (`self.ECurrentBallState`)
    (:`NewEnumerator5`
      ;[1 1 1] Add to Score
      (bind _output_get (set `self.CurrentHomeRunTotal` (+ (`self.CurrentHomeRunTotal`) 1)))
      (set `self.ECurrentBallState` "NewEnumerator1")
      (`KismetSystemLibrary.PrintString` (`KismetStringLibrary.Conv_IntToString` _output_get) true true (struct :`R` 0.920019 :`G` 1.0 :`A` 1.0)))))

(fn `UserConstructionScript`)